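; DefaultPlayer is the playable character Blueprint, handling action montages, a skill window and projectile spawning.
; Q plays the drink montage, while the AnimPlay and Act events share one normal-attack montage path.
; K toggles a newly created skill widget, switching input mode and cursor visibility with it.
; Helper functions spawn a given class at the actor's transform with a short lifespan and return player zero's pawn.
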(event EventBeginPlay)

(event Collision|EventActorBeginOverlap
  (params (OtherActor :type Actor%20Object%20Reference)))

(event EventTick
  (params (DeltaSeconds :type Float%20%28single-precision%29)))

(event EventAct
  (Development|PrintString "Act()")
  (Animation|Montage|PlayMontage (Variables|Character|GetMesh) "/Game/AllMaster/Playable/Animations/AM_NormalAttack.AM_NormalAttack"))

(event EventAnimPlay
  (params (number :type Integer))
  (Development|PrintString "Act()")
  (Animation|Montage|PlayMontage (Variables|Character|GetMesh) "/Game/AllMaster/Playable/Animations/AM_NormalAttack.AM_NormalAttack"))

(event Input|KeyboardEvents|Q
  (params (Key :type Key%20Structure :default "None"))
  (:Pressed
    (Animation|Montage|PlayMontage (Variables|Character|GetMesh) "/Game/AllMaster/Playable/Animations/AM_Drink.AM_Drink"
      (:then
        (Development|PrintString "Hello")))))

(event Input|KeyboardEvents|K
  (params (Key :type Key%20Structure :default "None"))
  (:Pressed
    (if (not (Variables|Default|GetbOnSkillWindow))
      (bind _returnvalue (UserInterface|CreateWidget "/Game/AllMaster/UI/WBP_SkillWindow.WBP_SkillWindow_C"))
      (bind _output_get (Variables|Default|SetSkillWindow _returnvalue))
      (UserInterface|Viewport|AddtoViewport _output_get 0)
      (Input|SetInputModeGameandUI (Game|GetPlayerController 0) 0 "DoNotLock" true)
      (Variables|Default|SetbOnSkillWindow true)
      (else
        (Widget|RemovefromParent (Variables|Default|GetSkillWindow))
        (Input|SetInputModeGameOnly (Game|GetPlayerController 0))
        (Variables|Default|SetbOnSkillWindow false)))
    (Variables|/Script/Engine.PlayerController|SetbShowMouseCursor (Game|GetPlayerController 0) (Variables|Default|GetbOnSkillWindow))))

(fn ConstructionScript)

(fn SpawnProjectiles
  (params (NewParam :type Projectile%20Class%20Reference))
  (bind _returnvalue (Game|SpawnActorfromClass NewParam (Transformation|GetActorTransform) "AdjustIfPossibleButAlwaysSpawn" 0 0))
  (Actor|SetLifeSpan _returnvalue 3.0))

(fn RetrunPlayer
  (return (Game|Player|GetPlayerPawn 0)))